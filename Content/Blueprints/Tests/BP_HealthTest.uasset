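; BP_HealthTest is a functional test that checks the DecreaseHealth function on FirstPersonCharacter.
; After a one-second delay, it casts player zero's character, records Health, then calls DecreaseHealth with the Damage variable.
; It succeeds only if the returned value exactly equals the recorded health minus Damage, fails otherwise, and reports an error if the cast fails.
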(event EventStartTest
  (bind _damage (Variables|Default|GetDamage))
  (Utilities|FlowControl|Delay 1.0)
  (bind _asfirst_person_character (Utilities|Casting|CastToFirstPersonCharacter (Game|GetPlayerCharacter 0))
    (:then
      (bind _output_get (Variables|Default|SetHealth (Variables|/Game/FirstPersonBP/Blueprints/FirstPersonCharacter.FirstPersonCharacter_C|GetHealth _asfirst_person_character)))
      (bind _health (Default|DecreaseHealth _asfirst_person_character _damage))
      (if (== _health (- _output_get _damage))
        (Class|FunctionalTest|FinishTest "Succeeded" "Damage Function Works")
        (else
          (Class|FunctionalTest|FinishTest "Failed" "Damage Function Failed"))))
    (:CastFailed
      (Class|FunctionalTest|FinishTest "Error" "Player cast failed"))))

(event EventTick
  (params (DeltaSeconds :type Float%20%28single-precision%29)))

(fn ConstructionScript)