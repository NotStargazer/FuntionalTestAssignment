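; BP_Alien is an enemy alien that melees the player and awards score when killed.
; Tick plays an attack montage when the living player is within range, pausing movement until it completes.
; DamagePlayer applies hit damage but is not called within this Blueprint.
; AnyDamage reduces health; death disables movement and collision, updates player score and multiplier, notifies either Mars game mode, then destroys the actor after a delay.
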(event EventBeginPlay)

(event Game|Damage|EventAnyDamage
  (params (Damage :type Float%20%28single-precision%29) (DamageType :type Damage%20Type%20Object%20Reference) (InstigatedBy :type Controller%20Object%20Reference) (DamageCauser :type Actor%20Object%20Reference))
  (bind _health (CallFunction|DecreaseHealth Damage))
  (if (<= _health 0.0)
    (CallFunction|KillAI)
    (Utilities|FlowControl|Delay 3.0)
    (Actor|DestroyActor)))

(event EventTick
  (params (DeltaSeconds :type Float%20%28single-precision%29))
  (bind _asfirst_person_character (Utilities|Casting|CastToFirstPersonCharacter (Game|GetPlayerCharacter 0)))
  (if (Math|Boolean|ANDBoolean (Default|IsAlive _asfirst_person_character) (and (not (CallFunction|IsAttacking)) (CallFunction|IsWithinAttackRange)) (CallFunction|IsAlive))
    (Components|Activation|Deactivate (Variables|Character|GetCharacterMovement))
    (Animation|Montage|PlayMontage (Variables|Character|GetMesh) "/Game/Characters/Enemy_Great_Spider/Animations/AlienAttack1.AlienAttack1"
      (:OnCompleted
        (Components|Activation|Activate (Variables|Character|GetCharacterMovement) false)))))

(fn ConstructionScript)

(fn IsWithinAttackRange
  (return (< (Transformation|GetDistanceTo (Game|GetPlayerCharacter 0)) (Variables|Default|GetAttack%20Range))))

(fn IsAttacking
  (return (Animation|Montage|MontageIsPlaying (Components|SkeletalMesh|GetAnimInstance (Variables|Character|GetMesh)) 0)))

(fn DamagePlayer
  (if (CallFunction|IsAlive)
    (Game|Damage|ApplyDamage (Game|GetPlayerCharacter 0) (Variables|Default|GetDamage%20Per%20Hit) 0 0)))

(fn DecreaseHealth
  (params (Damage :type Float%20%28single-precision%29))
  (bind _output_get (Variables|Default|SetHealth (- (Variables|Default|GetHealth) Damage)))
  (return _output_get))

(fn KillAI
  (bind _returnvalue (Game|GetGameMode))
  (bind _self self)
  (bind _charactermovement (Variables|Character|GetCharacterMovement))
  (Variables|Default|SetDead true)
  (Components|Activation|Deactivate _charactermovement)
  (Components|Movement|StopMovementImmediately _charactermovement)
  (Collision|SetActorEnableCollision false)
  (bind _asfirst_person_character (Utilities|Casting|CastToFirstPersonCharacter (Game|GetPlayerCharacter 0)))
  (Default|IncreaseScore _asfirst_person_character (Variables|Default|GetScore%20For%20Kill))
  (Default|UpdateMultiplier _asfirst_person_character false)
  (bind _asbp_mars_game_mode (Utilities|Casting|CastToBP_Mars_GameMode _returnvalue)
    (:then
      (Default|RegisterAlienDeath _asbp_mars_game_mode _self))
    (:CastFailed
      (bind _asbp_mars_test_gamemode (Utilities|Casting|CastToBP_Mars_TestGamemode _returnvalue))
      (Default|RegisterAlienDeath _asbp_mars_test_gamemode _self))))

(fn IsAlive
  (return (not (Variables|Default|GetDead))))