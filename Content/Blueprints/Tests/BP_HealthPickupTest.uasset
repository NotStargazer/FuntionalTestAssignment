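; Functional test that checks whether BP_HealthPickup heals the player.
; After a short delay, PrepareTest spawns the pickup at the test actor's transform, lowers the FirstPersonCharacter's Health to a known baseline, or errors if the cast fails.
; Tick then waits for the pickup to become invalid and passes only if Health has risen above that baseline.
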(event EventTick
  (params (DeltaSeconds :type Float%20%28single-precision%29))
  (if (Variables|Default|GetRun)
    (Utilities|IsValid (Variables|Default|GetHealth%20Pickup)
      (:Is%20Not%20Valid
        (if (> (Variables|/Game/FirstPersonBP/Blueprints/FirstPersonCharacter.FirstPersonCharacter_C|GetHealth (Variables|Default|GetPlayer)) (Variables|Default|GetStartHealth))
          (Class|FunctionalTest|FinishTest "Succeeded" "Healed the player successfully")
          (else
            (Class|FunctionalTest|FinishTest "Failed" "Player Not Healed")))))))

(event EventPrepareTest
  (Utilities|FlowControl|Delay 2.0)
  (bind _returnvalue (Game|SpawnActorfromClass "/Game/Blueprints/Picksups/BP_HealthPickup.BP_HealthPickup_C" (Transformation|GetActorTransform) "Undefined" 0 0))
  (bind _asfirst_person_character (Utilities|Casting|CastToFirstPersonCharacter (Game|GetPlayerCharacter 0))
    (:then
      (Variables|Default|SetHealth%20Pickup _returnvalue)
      (bind _output_get (Variables|Default|SetPlayer _asfirst_person_character))
      (Variables|/Game/FirstPersonBP/Blueprints/FirstPersonCharacter.FirstPersonCharacter_C|SetHealth _output_get 5e+01)
      (Variables|Default|SetStartHealth (Variables|/Game/FirstPersonBP/Blueprints/FirstPersonCharacter.FirstPersonCharacter_C|GetHealth _output_get))
      (Variables|Default|SetRun true))
    (:CastFailed
      (Class|FunctionalTest|FinishTest "Error" "Failed to Cast to player"))))

(fn ConstructionScript)