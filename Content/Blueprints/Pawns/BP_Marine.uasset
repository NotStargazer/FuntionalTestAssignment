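; BP_Marine is the player pawn: a marine with world-axis movement, a hitscan assault rifle, health and score.
; Each tick, mouse velocity above a deadzone sets a yaw that the control rotation smoothly interpolates toward.
; Firing starts effects, sound and a looping timer that line-traces from the muzzle along control rotation, applying damage.
; Taking damage resets the clamped score multiplier; zero health sets Dead, blocking movement, aiming and firing.
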(event EventTick
  (params (DeltaSeconds :type Float%20%28single-precision%29))
  (CallFunction|UpdatePlayerAim))

(event EventBeginPlay
  (bind _returnvalue (UserInterface|CreateWidget "/Game/UI/W_PlayerHUD.W_PlayerHUD_C" 0 self))
  (UserInterface|Viewport|AddtoViewport _returnvalue 0))

(event Game|Damage|EventAnyDamage
  (params (Damage :type Float%20%28single-precision%29) (DamageType :type Damage%20Type%20Object%20Reference) (InstigatedBy :type Controller%20Object%20Reference) (DamageCauser :type Actor%20Object%20Reference))
  (bind _health (CallFunction|DecreaseHealth Damage))
  (if (<= _health 0.0)
    (CallFunction|StopFiringWeapon)
    (Variables|Default|SetDead true)))

(event Input|ActionEvents|InputActionFireWeapon
  (params (Key :type Key%20Structure :default "None"))
  (:Pressed
    (CallFunction|StartFiringWeapon))
  (:Released
    (if (Components|Activation|IsActive (Variables|Default|GetP_AssaultRifle_MF))
      (CallFunction|StopFiringWeapon))))

(event Input|AxisEvents|InputAxisForward
  (params (AxisValue :type Float%20%28single-precision%29))
  (if (CallFunction|IsAlive)
    (Pawn|Input|AddMovementInput "1.000000, 0, 0" AxisValue false)))

(event Input|AxisEvents|InputAxisRight
  (params (AxisValue :type Float%20%28single-precision%29))
  (if (CallFunction|IsAlive)
    (Pawn|Input|AddMovementInput "0.000000,1.000000, 0" AxisValue false)))

(fn ConstructionScript)

(fn GetMouseVelocity
  (bind _returnvalue (Game|GetPlayerController 0))
  (bind (_deltax _deltay) (Class|PlayerController|GetInputMouseDelta _returnvalue))
  (return (/ (Math|Vector2D|MakeVector2D _deltax _deltay) (Utilities|Time|GetWorldDeltaSeconds))))

(fn UpdatePlayerAim
  (bind _returnvalue (Game|GetPlayerController 0))
  (bind _returnvalue_2 (CallFunction|GetMouseVelocity))
  (if (and (CallFunction|IsMouseAboveDeadzone) (CallFunction|IsAlive))
    (Pawn|SetControlRotation _returnvalue (Math|Interpolation|RInterpTo (Pawn|GetControlRotation _returnvalue :!class /Script/Engine.Controller) (Math|Rotator|MakeRotator 0.0 0.0 (Class|KismetMathLibrary|DegAtan2 (.x _returnvalue_2) (.y _returnvalue_2))) (Utilities|Time|GetWorldDeltaSeconds) (Variables|Default|GetMouseSmoothSpeed)))))

(fn IsMouseAboveDeadzone
  (return (> (Math|Vector2D|Vector2DLength (CallFunction|GetMouseVelocity)) (Variables|Default|GetMouse%20Deadzone))))

(fn StartFiringWeapon
  (if (CallFunction|IsAlive)
    (Components|Activation|Activate (Variables|Default|GetP_AssaultRifle_MF) false)
    (bind _returnvalue (Audio|SpawnSound2D "/Game/Sounds/Weapon_AssaultRifle/Stereo/RifleFire_Cue.RifleFire_Cue" 1.0 1.0 0.0 0))
    (Variables|Default|SetWeapon%20Fire%20Sound _returnvalue)
    (CallFunction|WeaponTrace)
    (Utilities|Time|SetTimerbyFunctionName 0 "Weapon Trace" (Variables|Default|GetWeapon%20Fire%20Rate) true)))

(fn StopFiringWeapon
  (if (CallFunction|IsAlive)
    (Components|Activation|Deactivate (Variables|Default|GetP_AssaultRifle_MF))
    (Audio|Components|Audio|Stop (Variables|Default|GetWeapon%20Fire%20Sound))
    (Utilities|Time|ClearTimerbyFunctionName 0 "Weapon Trace")
    (Audio|SpawnSound2D "/Game/Sounds/Weapon_AssaultRifle/Stereo/RifleFireEnd_Cue.RifleFireEnd_Cue" 1.0 1.0 0.0 0)))

(fn DecreaseHealth
  (params (Damage :type Float%20%28single-precision%29))
  (bind _output_get (Variables|Default|SetHealth (- (Variables|Default|GetHealth) Damage)))
  (CallFunction|UpdateMultiplier true)
  (return _output_get))

(fn IsAlive
  (return (not (Variables|Default|GetDead))))

(fn WeaponTrace
  (bind _outhit (Collision|LineTraceByChannel (CallFunction|GetWeaponTraceStartLocation) (CallFunction|GetWeaponTracerEndLocation) "TraceTypeQuery1" false 0 "None"))
  (if (.bBlockingHit (Collision|BreakHitResult _outhit))
    (CallFunction|SpawnImpactHit (.ImpactPoint (Collision|BreakHitResult _outhit)))
    (Game|Damage|ApplyDamage (.HitActor (Collision|BreakHitResult _outhit)) (Variables|Default|GetBase%20Damage) 0 0)))

(fn GetWeaponTraceStartLocation
  (return (Transformation|GetSocketLocation (Variables|Default|GetRifle) "MuzzleFlash")))

(fn GetWeaponTracerEndLocation
  (return (+ (CallFunction|GetWeaponTraceStartLocation) (* (Math|Vector|GetForwardVector (Pawn|GetControlRotation :!class /Script/Engine.Pawn)) (Variables|Default|GetWeapon%20Range)))))

(fn IncreaseScore
  (params (Score%20For%20Kill :type Integer))
  (bind _output_get (Variables|Default|SetScore (+ (Variables|Default|GetScore) (* Score%20For%20Kill (Variables|Default|GetMultiplier)))))
  (return _output_get))

(fn UpdateMultiplier
  (params (Reset :type Boolean))
  (if Reset
    (bind _output_get (Variables|Default|SetMultiplier 1))
    (return _output_get)
    (else
      (bind _result (Math|Integer|IncrementInt (Variables|Default|GetMultiplier))
        (:%20%20
          (bind _output_get_2 (Variables|Default|SetMultiplier (Math|Integer|Clamp(Integer) _result 1 4)))
          (return _output_get_2))))))

(fn SpawnImpactHit
  (params (Hit%20Location :type Vector))
  (Effects|SpawnEmitteratLocation "/Game/Effects/Weapons/Impacts/P_AssaultRifle_IH.P_AssaultRifle_IH" Hit%20Location))

(fn AddHealth
  (params (Health :type Float%20%28single-precision%29))
  (bind _output_get (Variables|Default|SetHealth (Math|Float|Clamp(Float) (+ Health (Variables|Default|GetHealth)) 0.0 1e+02)))
  (return _output_get))

(fn IsHealthFull
  (return (>= (Variables|Default|GetHealth) 1e+02)))