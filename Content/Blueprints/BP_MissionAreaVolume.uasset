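; BP_MissionAreaVolume is a mission boundary volume that punishes the player for leaving the playable area.
; When a FirstPersonCharacter exits the CollisionArea, it sets the character's OutsideMissionArea flag and starts a Kill Player timer lasting SecondsBeforePlayerDeath.
; Re-entering clears the flag and cancels the timer.
; If the timer fires, Kill Player applies fixed damage to player character 0 rather than the character that left.
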(event OnComponentBeginOverlap(CollisionArea)
  (params (OverlappedComponent :type Primitive%20Component%20Object%20Reference) (OtherActor :type Actor%20Object%20Reference) (OtherComp :type Primitive%20Component%20Object%20Reference) (OtherBodyIndex :type Integer) (bFromSweep :type Boolean) (SweepResult :type Hit%20Result%20Structure%20%28by%20ref%29))
  (bind _asfirst_person_character (Utilities|Casting|CastToFirstPersonCharacter OtherActor))
  (Variables|/Game/FirstPersonBP/Blueprints/FirstPersonCharacter.FirstPersonCharacter_C|SetOutside%20Mission%20Area _asfirst_person_character false)
  (Utilities|Time|ClearTimerbyFunctionName self "Kill Player"))

(event OnComponentEndOverlap(CollisionArea)
  (params (OverlappedComponent :type Primitive%20Component%20Object%20Reference) (OtherActor :type Actor%20Object%20Reference) (OtherComp :type Primitive%20Component%20Object%20Reference) (OtherBodyIndex :type Integer))
  (bind _asfirst_person_character (Utilities|Casting|CastToFirstPersonCharacter OtherActor))
  (Variables|/Game/FirstPersonBP/Blueprints/FirstPersonCharacter.FirstPersonCharacter_C|SetOutside%20Mission%20Area _asfirst_person_character true)
  (Utilities|Time|SetTimerbyFunctionName self "Kill Player" (Variables|Default|GetSeconds%20before%20player%20death)))

(fn ConstructionScript)

(fn KillPlayer
  (Game|Damage|ApplyDamage (Game|GetPlayerCharacter 0) 1e+02 0 0))