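; BP_WaveTest is a functional test for the alien wave system in the Mars test game mode.
; PrepareTest casts the game mode to BP_Mars_TestGamemode, calls SetupNewWave and arms the Tick check.
; Tick passes the test once AliensLeftToKill reaches zero or below, despite the "spawned successfully" message, and reports an error if the stored game mode becomes invalid.
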(event EventTick
  (params (DeltaSeconds :type Float%20%28single-precision%29))
  (bind _gamemode (Variables|Default|GetGamemode))
  (if (Variables|Default|GetStart%20Test)
    (Utilities|IsValid _gamemode
      (:Is%20Valid
        (if (<= (Variables|/Game/Blueprints/GameMode/BP_Mars_TestGamemode.BP_Mars_TestGamemode_C|GetAliens%20Left%20To%20Kill _gamemode) 0)
          (Class|FunctionalTest|FinishTest "Succeeded" "Wave spawned successfully")))
      (:Is%20Not%20Valid
        (Class|FunctionalTest|FinishTest "Error" "Gamemode not valid")))))

(event EventPrepareTest
  (bind _asbp_mars_test_gamemode (Utilities|Casting|CastToBP_Mars_TestGamemode (Game|GetGameMode)))
  (bind _output_get (Variables|Default|SetGamemode _asbp_mars_test_gamemode))
  (Default|SetupNewWave _output_get)
  (Variables|Default|SetStart%20Test true))

(fn ConstructionScript)