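; Functional test that checks an alien can kill the player.
; On test start it casts the player to FirstPersonCharacter, lowers its health, disables movement and shooting, and spawns a BP_Alien at the test actor's transform.
; Tick polls the stored player and finishes the test as succeeded once it is no longer alive, with no explicit failure branch in the graph.
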(event EventStartTest
  (bind _asfirst_person_character (Utilities|Casting|CastToFirstPersonCharacter (Game|GetPlayerCharacter 0)))
  (Variables|/Game/FirstPersonBP/Blueprints/FirstPersonCharacter.FirstPersonCharacter_C|SetHealth _asfirst_person_character 2e+01)
  (Variables|/Game/FirstPersonBP/Blueprints/FirstPersonCharacter.FirstPersonCharacter_C|SetCan%20Move _asfirst_person_character false)
  (Variables|/Game/FirstPersonBP/Blueprints/FirstPersonCharacter.FirstPersonCharacter_C|SetCan%20Shoot _asfirst_person_character false)
  (Variables|Default|SetPlayer _asfirst_person_character)
  (Game|SpawnActorfromClass "/Game/Blueprints/AI/BP_Alien.BP_Alien_C" (Transformation|GetActorTransform) "Undefined" 0 0))

(event EventTick
  (params (DeltaSeconds :type Float%20%28single-precision%29))
  (if (not (Default|IsAlive (Variables|Default|GetPlayer)))
    (Class|FunctionalTest|FinishTest "Succeeded" "Player is dead")))

(fn ConstructionScript)