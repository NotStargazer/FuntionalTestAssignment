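; Test game mode for a Mars wave shooter that manages alien waves, with wave end still unimplemented.
; Each wave setup raises the alien count and starts a looping timer that spawns aliens at random TargetPoints until the quota is spent.
; Alien deaths update tracking and may drop a health pickup, likelier as player health falls.
; The completion check triggers nothing, and nothing here calls wave setup.
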(event Custom|Spawn%20Wave
  (CallFunction|SpawnAlien))

(event Custom|End%20Wave)

(fn ConstructionScript)

(fn SetupNewWave
  (Math|Integer|IncrementInt (Variables|Default|GetCurrent%20Wave)
    (:%20%20
      (Utilities|Time|SetTimerbyFunctionName 0 "Spawn Wave" 1.0 true)
      (CallFunction|IncreaseWaveDiffculty))))

(fn SpawnAlien
  (bind _spawn_point (CallFunction|GetRandomSpawnPoint))
  (Utilities|IsValid _spawn_point
    (:Is%20Valid
      (bind _returnvalue (Game|SpawnActorfromClass "/Game/Blueprints/AI/BP_Alien.BP_Alien_C" (Transformation|GetActorTransform _spawn_point) "Undefined" 0 0))
      (Development|PrintString "Enemy Spawn")
      (Utilities|IsValid _returnvalue
        (:Is%20Valid
          (Utilities|Array|Add (Variables|Default|GetAliens) _returnvalue)
          (bind _result (Math|Integer|DecrementInt (Variables|Default|GetAlien%20Spawns%20Remaining))
            (:%20%20
              (if (== _result 0)
                (Utilities|Time|ClearTimerbyFunctionName 0 "Spawn Wave")))))))))

(fn GetRandomSpawnPoint
  (bind _outactors (Actor|GetAllActorsOfClass "/Script/Engine.TargetPoint"))
  (return (Utilities|Array|Get(acopy) _outactors (Math|Random|RandomIntegerinRange 0 (Utilities|Array|LastIndex _outactors)))))

(fn RegisterAlienDeath
  (params (Alien :type BP%20Alien%20Object%20Reference%20%28by%20ref%29))
  (bind _asfirst_person_character (Utilities|Casting|CastToFirstPersonCharacter (Game|GetPlayerCharacter 0)))
  (if (> (- 1e+02 (Variables|/Game/FirstPersonBP/Blueprints/FirstPersonCharacter.FirstPersonCharacter_C|GetHealth _asfirst_person_character)) (+ (* 100 (Math|Random|RandomFloat)) 25.0))
    (Game|SpawnActorfromClass "/Game/Blueprints/Picksups/BP_HealthPickup.BP_HealthPickup_C" (Transformation|GetActorTransform Alien) "Undefined" 0 0))
  (Utilities|Array|RemoveItem (Variables|Default|GetAliens) Alien)
  (Math|Integer|DecrementInt (Variables|Default|GetAliens%20Left%20To%20Kill)
    (:%20%20
      (if (CallFunction|IsWaveComplete)
        _))))

(fn IsWaveComplete
  (return (and (== (Utilities|Array|Length (Variables|Default|GetAliens)) 0) (== (Variables|Default|GetAlien%20Spawns%20Remaining) 0))))

(fn IncreaseWaveDiffculty
  (bind _output_get (Variables|Default|SetAliens%20This%20Wave (+ (Variables|Default|GetAliens%20This%20Wave) 2)))
  (bind _output_get_2 (Variables|Default|SetAliens%20Left%20To%20Kill _output_get))
  (Variables|Default|SetAlien%20Spawns%20Remaining _output_get_2))